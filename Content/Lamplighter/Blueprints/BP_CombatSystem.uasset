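; Combat component for the player that handles combo attacks and dodge rolls on the owning BP_Player's mesh.
; Attack presses queue montage indices in a FIFO, cycling through AttacksAnim, and start playback when idle.
; The attack-animation-end event plays the next queued attack or resets the combo.
; Attack start and end events toggle CanDodge, which gates the roll montage, while DoOnce nodes guard both actions against re-entry during their short delays.
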(event `InitializeCombatSystem`
  ;[0.01042 0.01042 0.01042 1 33] Initialize Combat System
  (if (not (`KismetSystemLibrary.IsValid` (`self.PlayerMesh`)))
    (bind _asbp_player (cast `/Game/Lamplighter/Blueprints/BP_Player` (`self.GetOwner`)))
    (set `self.PlayerMesh` (`Character.Mesh` _asbp_player)))
  (set `self.AttackIndex` 0)
  (set `self.CanAttack` true)
  (set `self.AnimationInProgress` false)
  (`KismetArrayLibrary.Array_Clear` (`self.AttacksFifo`))
  (if (> (`KismetArrayLibrary.Array_Length` (`self.AttacksAnim`)) 0)
    _))

(event `Attack`
  ;[0 0 0 1 33] Attack
  (`/Engine/EditorBlueprintResources/StandardMacros.DoOnce` false :!label _label
    (:`Completed`
      (set `self.AnimationInProgress` true)
      (`KismetSystemLibrary.Delay` 0.1)
      (`|PlayMontage` (`self.PlayerMesh`) (`|GetArrayItem` (`self.AttacksAnim`) (`|GetArrayItem` (`self.AttacksFifo`)))
        (:`then`
          (`KismetArrayLibrary.Array_Remove` (`self.AttacksFifo`))
          (goto _label :!via `Reset`))))))

(event `OnAttackButtonStart`
  ;[0 0 0 1 33] OnAttackButtonStart
  (if (`self.CanAttack`)
    (if (`self.AnimationInProgress`)
      (`self.AddAttackToFifo` (`self.AttackIndex`))
      (else
        (`self.AddAttackToFifo` 0)
        (`self.Attack`)))))

(event `OnDodgeButtonStart`
  ;[0 0 0] Dodge
  (if (`self.CanDodge`)
    (`/Engine/EditorBlueprintResources/StandardMacros.DoOnce` false :!label _label_2
      (:`Completed`
        (`KismetSystemLibrary.Delay` 0.1)
        (`|PlayMontage` (`self.PlayerMesh`) "/Game/Lamplighter/AnimationsMixamo/SprintingForwardRoll_UE_Montage.SprintingForwardRoll_UE_Montage"
          (:`then`
            (goto _label_2 :!via `Reset`)))))))

(event `OnAttackAnimationStart`
  ;[0 0 0 1 33] OnAttackAnimationStart
  (set `self.CanDodge` false))

(event `OnAttackAnimationEnd`
  ;[0 0 0 1 33] OnAttackAnimationEnd
  (set `self.CanDodge` true)
  (if (> (`KismetArrayLibrary.Array_Length` (`self.AttacksFifo`)) 0)
    (`self.Attack`)
    (else
      (`self.StopCombo`))))

(event `StopCombo`
  ;[0 0 0 1 33] StopCombo
  (set `self.AnimationInProgress` false)
  (set `self.AttackIndex` 0)
  (if (> (`KismetArrayLibrary.Array_Length` (`self.AttacksFifo`)) 0)
    (`KismetArrayLibrary.Array_Clear` (`self.AttacksFifo`)))
  (set `self.CanAttack` true))

(fn `AddAttackToFifo`
  (params (attackIndex :type Integer))
  (`KismetArrayLibrary.Array_Add` (`self.AttacksFifo`) attackIndex)
  (`self.IncrementAttackIndex`))

(fn `IncrementAttackIndex`
  (set `self.AttackIndex` (mod (+ (`self.AttackIndex`) 1) (`KismetArrayLibrary.Array_Length` (`self.AttacksAnim`)))))